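; Actor component that gives its owner a drop shadow on the surface below it.
; On BeginPlay it spawns a BP_DropShadow actor, then repositions it every tick with a long downward Visibility trace from the owner.
; The shadow sits slightly above the impact point, rotated by a look-at between its up vector and the surface normal, with no check for a missed trace.
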(event EventBeginPlay
  (bind _returnvalue (Game|SpawnActorfromClass "/Game/Blueprints/BP_DropShadow.BP_DropShadow_C" (Transformation|GetActorTransform (Components|GetOwner)) "Undefined" "MultiplyWithRoot" 0 0))
  (Variables|Default|SetDropShadow _returnvalue)
  (CallFunction|UpdateShadowTransform))

(event EventTick
  (params (DeltaSeconds :type Float%20%28single-precision%29))
  (CallFunction|UpdateShadowTransform))

(fn UpdateShadowTransform
  (bind _returnvalue (Components|GetOwner))
  (bind _dropshadow (Variables|Default|GetDropShadow))
  (bind _returnvalue_2 (Transformation|GetActorLocation _returnvalue))
  (bind _returnvalue_3 (+ _returnvalue_2 "0.000000,0.000000,0.100000"))
  (bind _outhit (Collision|LineTraceByChannel _returnvalue_3 (+ _returnvalue_3 "0.000000,0.000000,-10000.000000") "TraceTypeQuery1" false 0 "None"))
  (Transformation|SetActorLocation _dropshadow (+ (.ImpactPoint (Collision|BreakHitResult _outhit)) "0.000000,0.000000,2.000000") false false)
  (Transformation|SetActorRotation _dropshadow (Math|Rotator|FindLookatRotation (Transformation|GetActorUpVector _dropshadow) (.ImpactNormal (Collision|BreakHitResult _outhit)))))