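; BP_GeoSpawnSwitch is an interactable switch that reveals a referenced piece of geometry.
; On BeginPlay it hides GeoToSpawn and disables its collision, so the geometry is already placed and only toggled, not spawned.
; OnInteract makes it visible and collidable again and sets the Sphere component to a fixed relative position, with no path to revert.
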(event EventBeginPlay
  (bind _geotospawn (Variables|Default|GetGeoToSpawn))
  (|CallParentFunction)
  (Collision|SetActorEnableCollision _geotospawn false)
  (Rendering|SetActorHiddenInGame _geotospawn true))

(event Collision|EventActorBeginOverlap
  (params (OtherActor :type Actor%20Object%20Reference)))

(event EventTick
  (params (DeltaSeconds :type Float%20%28single-precision%29))
  (|CallParentFunction DeltaSeconds) ; This node is disabled and will not be called.\nDrag off pins to build functionality.
)

(event EventOnInteract
  (bind _geotospawn (Variables|Default|GetGeoToSpawn))
  (Collision|SetActorEnableCollision _geotospawn true)
  (Rendering|SetActorHiddenInGame _geotospawn false)
  (Transformation|SetRelativeLocation (Variables|Default|GetSphere) "0.000000,0.000000,15.000000" false false))

(fn ConstructionScript
  (|CallParentFunction))